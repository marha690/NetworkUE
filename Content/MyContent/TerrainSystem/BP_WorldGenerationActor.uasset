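; World generation actor that manages terrain tiles around players and exposes an event for changing terrain height within a radius.
; On the authority, a looping one-second timer adds and removes tiles around the player.
; Listen or standalone hosts and remote clients register their first player pawn for tracking at BeginPlay, while dedicated servers skip this.
; The tile, tracking and height logic live outside this graph, which only calls them.
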(event Custom|ChangeTerrainHeight
  (params (Position :type Vector) (Radius :type Float%20%28single-precision%29) (AdditionalHeight :type Float%20%28single-precision%29))
  (Class|ProceduralWorldLevelScript|UpdateTerrainHeight Position Radius AdditionalHeight))

(event Custom|UpdateTerrain
  (Class|ProceduralWorldLevelScript|AddTilesAroundPlayer)
  (Class|ProceduralWorldLevelScript|RemoveTilesAroundPlayer))

(event EventBeginPlay
  (Networking|SwitchHasAuthority
    (:Authority
      (Utilities|Time|SetTimerbyEvent (delegate Custom|UpdateTerrain) 1.0 true)
      (if (not (Networking|IsDedicatedServer))
        (Class|ProceduralWorldLevelScript|TrackPlayer (Game|Player|GetPlayerPawn 0) :!label _label)
        (Development|PrintString "Tracks player")))
    (:Remote
      (goto _label))))

(fn ConstructionScript)