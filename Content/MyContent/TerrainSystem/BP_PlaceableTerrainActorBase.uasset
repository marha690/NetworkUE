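; Base actor for placeable terrain objects that snaps itself vertically onto the generated world's terrain.
; On BeginPlay, if IsRoot is set, it queries BP_WorldGenerationActor for the height at its position, keeps X and Y, and moves to that height.
; The result is stored in Location, whose RepNotify moves the actor with sweep enabled, unlike the initial unswept move.
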(event Custom|SetHeightToTerrain
  (bind _returnvalue (Transformation|GetActorLocation))
  (bind (_x _y) (Math|Vector|BreakVector _returnvalue))
  (if (Variables|Default|GetIsRoot?)
    (bind _returnvalue_2 (Actor|GetActorOfClass "/Game/MyContent/TerrainSystem/BP_WorldGenerationActor.BP_WorldGenerationActor_C"))
    (bind _height (Class|ProceduralWorldLevelScript|GetHeight _returnvalue_2 _returnvalue))
    (bind _output_get (Variables|Default|SetLocation (Math|Vector|MakeVector _x _y _height)))
    (Transformation|SetActorLocation self _output_get false false)))

(event EventBeginPlay
  (CallFunction|SetHeighttoTerrain))

(fn ConstructionScript)

(fn OnRepLocation
  (Transformation|SetActorLocation (Variables|Default|GetLocation) true false))